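; Player pawn Blueprint that handles movement and turning from keyboard, mouse and gamepad axis inputs.
; Keyboard and gamepad axes add movement along the control rotation's forward and right vectors.
; Mouse X adds controller yaw, which steers that movement.
; Gamepad X instead sets an absolute actor rotation from a quaternion with the axis value as X and W at 1, so it acts on roll, not yaw.
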(event `InputAxis|Forward_Backward`
  (params (AxisValue :type "Float (single-precision)"))
  ;[1 1 1] X-Y Axis Movement - Keyboard
  (`self.AddMovementInput` (`KismetMathLibrary.GetForwardVector` (`self.GetControlRotation`)) AxisValue))

(event `InputAxis|Rotate_Right_Left`
  (params (AxisValue :type "Float (single-precision)"))
  ;[1 1 1] Rotate With Mouse X - Keyboard
  (`self.AddControllerYawInput` AxisValue))

(event `InputAxis|Right_Left`
  (params (AxisValue :type "Float (single-precision)"))
  ;[1 1 1] X-Y Axis Movement - Keyboard
  (`self.AddMovementInput` (`KismetMathLibrary.GetRightVector` (`self.GetControlRotation`)) AxisValue))

(event `InputAxis|Rotate_Gamepad_X`
  (params (AxisValue :type "Float (single-precision)"))
  (`self.K2_SetActorRotation` (`KismetMathLibrary.Conv_Vector4ToRotator` (`KismetMathLibrary.MakeVector4` AxisValue 0.0 0.0 1.0))))

(event `InputAxis|Forward_Backward_GamePad`
  (params (AxisValue :type "Float (single-precision)"))
  (`self.AddMovementInput` (`KismetMathLibrary.GetForwardVector` (`self.GetControlRotation`)) AxisValue))

(event `InputAxis|Right_Left_Gamepad`
  (params (AxisValue :type "Float (single-precision)"))
  (`self.AddMovementInput` (`KismetMathLibrary.GetRightVector` (`self.GetControlRotation`)) AxisValue))

(fn `UserConstructionScript`)