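; Mark_Camera is a shared multiplayer camera actor that zooms according to how far apart two to four players are.
; On BeginPlay it caches the players from Mark_GameMode and sets itself as every PlayerController's view target.
; A fast looping timer, used instead of Tick, sets the spring arm length to the largest pairwise player distance, clamped between minimum and maximum limits.
; Only arm length is updated, not the camera's position.
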(event `self.ReceiveBeginPlay`
  (`self.ClassSetup`)
  (`KismetSystemLibrary.K2_SetTimer` null "UpdateCamera" 0.001 true))

(event `UpdateCamera`
  (switch `int` (`KismetArrayLibrary.Array_Length` (`self.PlayersReference`))
    (:`2`
      (`self.SetArmLength2Player`))
    (:`3`
      (`self.SetArmLength3Player`))
    (:`4`
      (`self.SetArmLength4Player`))))

(fn `ClassSetup`
  (bind _asmark_game_mode (cast `/Game/Blueprints/Mark_GameMode` (`GameplayStatics.GetGameMode`))
    (:`then`
      _)
    (:`CastFailed`
      _))
  (bind _output_get (set `self.Mark_GameMode` _asmark_game_mode))
  (set `self.PlayersReference` (`/Game/Blueprints/Mark_GameMode.Players` _output_get))
  (bind _outactors (`GameplayStatics.GetAllActorsOfClass` "/Script/Engine.PlayerController"))
  (`PlayerController.SetViewTargetWithBlend` _outactors self 0.0 "VTBlend_Linear" 0.0 false)
  (for (_array_element _array_index) (`self.PlayersReference`)
    (switch `int` _array_index
      (:`0`
        (set `self.Player1` _array_element))
      (:`1`
        (set `self.Player2` _array_element))
      (:`2`
        (set `self.Player 3` _array_element))
      (:`3`
        (set `self.Player 4` _array_element)))))

(fn `SetArmLength2Player`
  (set `SpringArmComponent.TargetArmLength` (`KismetMathLibrary.FClamp` (`self.GetDistanceTo` (`self.Player1`) (`self.Player2`)) (`self.MinArmLength`) (`self.MaxArmLength`)) (`self.SpringArm`)))

(fn `SetArmLength3Player`
  (bind _player1 (`self.Player1`))
  (bind _player2 (`self.Player2`))
  (bind _player_3 (`self.Player 3`))
  (set `SpringArmComponent.TargetArmLength` (`KismetMathLibrary.FClamp` (`.MaxValue` (`KismetMathLibrary.MaxOfFloatArray` (`|MakeArray` (`self.GetDistanceTo` _player1 _player2) (`self.GetDistanceTo` _player1 _player_3) (`self.GetDistanceTo` _player2 _player_3)))) (`self.MinArmLength`) (`self.MaxArmLength`)) (`self.SpringArm`)))

(fn `SetArmLength4Player`
  (bind _player1 (`self.Player1`))
  (bind _player2 (`self.Player2`))
  (bind _player_3 (`self.Player 3`))
  (bind _player_4 (`self.Player 4`))
  (set `SpringArmComponent.TargetArmLength` (`KismetMathLibrary.FClamp` (`.MaxValue` (`KismetMathLibrary.MaxOfFloatArray` (`|MakeArray` (`self.GetDistanceTo` _player1 _player2) (`self.GetDistanceTo` _player1 _player_3) (`self.GetDistanceTo` _player1 _player_4) (`self.GetDistanceTo` _player2 _player_3) (`self.GetDistanceTo` _player2 _player_4) (`self.GetDistanceTo` _player_3 _player_4)))) (`self.MinArmLength`) (`self.MaxArmLength`)) (`self.SpringArm`)))

(fn `UserConstructionScript`)