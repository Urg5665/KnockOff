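; AirProjectile is a short-lived projectile actor that uses character movement and destroys itself.
; On BeginPlay it resets a counter, re-applies its control rotation, prints it, and issues a single large movement input along that rotation's forward vector.
; Tick increments the counter and destroys the actor after about 50 frames, so lifetime depends on frame rate.
; No overlap or hit logic is active, and alternative location-offset and impulse movement nodes are left unconnected.
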(event `self.ReceiveBeginPlay`
  (bind _returnvalue (`self.GetControlRotation`))
  (set `self.TimeAlive` 0)
  (`Controller.SetControlRotation` (`self.GetController`) _returnvalue)
  (`KismetSystemLibrary.PrintString` (`KismetStringLibrary.Conv_RotatorToString` _returnvalue))
  (`KismetSystemLibrary.PrintString` (`KismetStringLibrary.Conv_RotatorToString` (`self.GetControlRotation`)))
  (`self.AddMovementInput` (`KismetMathLibrary.GetForwardVector` (`self.GetControlRotation`)) 50.0))

(event `self.ReceiveTick`
  (params (DeltaSeconds :type "Float (single-precision)"))
  (bind _output_get (set `self.TimeAlive` (+ (`self.TimeAlive`) 1)))
  (if (> _output_get 50)
    (`self.K2_DestroyActor`)))

(fn `UserConstructionScript`)