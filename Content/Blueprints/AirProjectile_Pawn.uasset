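; AirProjectile_Pawn is a projectile pawn that launches on spawn and destroys itself shortly afterwards.
; BeginPlay passes the forward vector of the pawn's own control rotation, scaled to a fixed speed, to ProjectileMovement as local-space velocity, and debug-prints that rotation twice.
; Tick counts frames rather than seconds and destroys the actor past a fixed count, so its lifetime varies with frame rate.
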(event `self.ReceiveBeginPlay`
  (set `self.TimeAlive` 0)
  (`KismetSystemLibrary.PrintString` (`KismetStringLibrary.Conv_RotatorToString` (`self.GetControlRotation`)))
  (`KismetSystemLibrary.PrintString` (`KismetStringLibrary.Conv_RotatorToString` (`self.GetControlRotation`)))
  (`ProjectileMovementComponent.SetVelocityInLocalSpace` (`self.ProjectileMovement`) (* (`KismetMathLibrary.GetForwardVector` (`self.GetControlRotation`)) 3000.0)))

(event `self.ReceiveTick`
  (params (DeltaSeconds :type "Float (single-precision)"))
  (bind _output_get (set `self.TimeAlive` (+ (`self.TimeAlive`) 1)))
  (if (> _output_get 50)
    (`self.K2_DestroyActor`)))

(fn `UserConstructionScript`)